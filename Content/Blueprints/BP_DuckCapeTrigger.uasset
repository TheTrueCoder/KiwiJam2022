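; BP_DuckCapeTrigger is a one-shot pickup trigger that upgrades the third-person player character to the DuckP4 mesh with extra jumps.
; When the player overlaps its box, it spawns a burst Niagara effect and sets the character's respawn transform to that location.
; It then raises the max jump count, swaps the skeletal mesh, launches the character upward and destroys itself.
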(event `self.Box.OnComponentBeginOverlap`
  (params (OverlappedComponent :type "PrimitiveComponent Object Reference") (OtherActor :type "Actor Object Reference") (OtherComp :type "PrimitiveComponent Object Reference") (OtherBodyIndex :type Integer) (bFromSweep :type Boolean) (SweepResult :type "HitResult Structure (by ref)"))
  (bind _returnvalue (`GameplayStatics.GetPlayerCharacter` 0))
  (bind _returnvalue_2 (`SceneComponent.K2_GetComponentLocation` (`self.Box`)))
  (if (== OtherActor _returnvalue)
    (bind _asbp_third_person_character (cast `/Game/Blueprints/BP_ThirdPersonCharacter` _returnvalue))
    (`NiagaraFunctionLibrary.SpawnSystemAtLocation` "/Game/VFX/vfx_burst.vfx_burst" _returnvalue_2)
    (set `/Game/Blueprints/BP_ThirdPersonCharacter.respawn` (`KismetMathLibrary.Conv_VectorToTransform` _returnvalue_2) _asbp_third_person_character)
    (set `Character.JumpMaxCount` 5 _asbp_third_person_character)
    (`SkinnedMeshComponent.SetSkinnedAssetAndUpdate` (`Character.Mesh` _asbp_third_person_character) "/Game/Characters/Duck/DuckP4.DuckP4" true)
    (`Character.LaunchCharacter` _asbp_third_person_character (0.0 0.0 800.0) false false)
    (`self.K2_DestroyActor`)))

(fn `UserConstructionScript`)